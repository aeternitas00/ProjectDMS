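; Card container for a BP_TestLocation that shows and lays out the cards placed at that location.
; Added cards attach to the location's player or enemy slot, depending on whether their owner ID resolves to a player in the DMS game state.
; Each side is arranged in a grid from row size and X/Y spacing.
; Removed cards are hidden and detached, and both sides are re-laid out.
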(event `self.OnContainerAdded`
  (params (AddedCards :type "Array of DMSSpawnableBase Object Reference (by ref)"))
  (bind _asbp_test_location (cast `/Game/DMSGame/Locations/BP_TestLocation` (`self.GetOwner`)))
  (for _array_element AddedCards
    (`Actor.SetActorHiddenInGame` _array_element false)
    (`/Engine/EditorBlueprintResources/StandardMacros.IsValid` (`DMSGameState.FindPlayerFromId` (`DMSGameMode.GetDMSGameState` (`DMSCoreFunctionLibrary.GetDMSGameMode` self)) (`DMSSpawnableBase.GetOwnerID` _array_element))
      (:`Is Valid`
        (`KismetArrayLibrary.Array_AddUnique` (`self.Child_PlayerSide`) _array_element)
        (`Actor.K2_AttachToComponent` _array_element (`/Game/DMSGame/Locations/BP_TestLocation.ChildSlot_Player` _asbp_test_location) "None" "KeepRelative" "KeepRelative" "KeepRelative" false)
        (`self.UpdateChildsOffset` (`self.Child_PlayerSide`)))
      (:`Is Not Valid`
        (`KismetArrayLibrary.Array_AddUnique` (`self.Child_EnemySide`) _array_element)
        (`Actor.K2_AttachToComponent` _array_element (`/Game/DMSGame/Locations/BP_TestLocation.ChildSlot_Enemy` _asbp_test_location) "None" "KeepRelative" "KeepRelative" "KeepRelative" false)
        (`self.UpdateChildsOffset` (`self.Child_EnemySide`))))))

(event `self.OnContainerRemoved`
  (params (RemovedCards :type "Array of DMSSpawnableBase Object Reference (by ref)"))
  (for _array_element RemovedCards
    (`KismetArrayLibrary.Array_RemoveItem` (`self.Child_PlayerSide`) _array_element)
    (`KismetArrayLibrary.Array_RemoveItem` (`self.Child_EnemySide`) _array_element)
    (`Actor.SetActorHiddenInGame` _array_element true)
    (`Actor.K2_DetachFromActor` _array_element "KeepRelative" "KeepRelative" "KeepRelative"))
  (`self.UpdateChildsOffset` (`self.Child_PlayerSide`))
  (`self.UpdateChildsOffset` (`self.Child_EnemySide`)))

(fn `UpdateChildsOffset`
  (params (Array :type "Array of Actor Object Reference (by ref)"))
  (locals (`Num Per Row` :type Integer :default 3) (DistanceX :type "Vector Structure" :default (0.0 140.0 0.0)) (DistanceY :type "Vector Structure" :default (-140.0 0.0 0.0)))
  (bind _num_per_row (`local.Num Per Row`))
  (for (_array_element _array_index) Array
    (`Actor.K2_SetActorRelativeLocation` _array_element (+ (* (`local.DistanceX`) (mod _array_index _num_per_row)) (* (`local.DistanceY`) (`KismetMathLibrary.Conv_IntToVector` (/ _array_index _num_per_row)))) false true)))