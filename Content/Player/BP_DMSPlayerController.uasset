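; Player controller for a DMS card game that sets up the player's HUD, attributes and card containers.
; The test HUD is built at construction, then shown with Game-and-UI input during DMS data setup.
; Selection changes toggle interaction widgets on owned cards, and a test event plays cards through DMS sequence manager effect sequences.
; A helper loads saved character and card data into the player state.
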(event `Setup DMS Datas`
  (bind _testhud (`self.TestHUD`))
  (`UserWidget.AddToViewport` _testhud 0)
  (`WidgetBlueprintLibrary.SetInputMode_GameAndUIEx` self _testhud "DoNotLock" false)
  (`self.SetupAttributes`)
  (`self.SetupCardContainers`)
  (`/Game/Widgets/WB_TestHUD.Setup Subwidget` (`self.TestHUD`)))

(event `self.ReceiveBeginPlay`
  (`parent.ReceiveBeginPlay`))

(event `self.PlayCard`
  (params (Card :type "DMSCardBase Object Reference"))
  (bind _returnvalue (`DMSCoreFunctionLibrary.GetDMSSequenceManager`))
  (bind _returnvalue_2 (`DMSSeqManager.RequestCreateSequence` _returnvalue self self (`BlueprintMapLibrary.Map_Find` (`self.DefaultBasicActions`) "PlayCard") (`|MakeArray` (cast `DMSEffectorInterface` Card :!pure true)) null null))
  (`DMSSeqManager.RunSequence` _returnvalue _returnvalue_2))

(event `self.OnSelectedObject`
  (params (FormerObject :type "Object Object Reference"))
  (`|ExecutionSequence`
    (:`then_0`
      (bind _asbp_card (`self.Check Object Is My Card` FormerObject)
        (:`then`
          (`/Game/Card/BP_Card.Close Interaction Widget` _asbp_card))))
    (:`then_1`
      (bind _asbp_card_2 (`self.Check Object Is My Card` (`self.SelectingObject`))
        (:`then`
          (`/Game/Card/BP_Card.Popup Interaction Widget` _asbp_card_2))))))

(fn `Load Client Save game`
  (returns (`Saved Card Datas` :type "Array of DMSCardData Structure") (`Player Character Data` :type "DMSPlayerCharacterData Structure"))
  (bind _returnvalue (`GameplayStatics.LoadGameFromSlot` (`self.Default Slot Name`)))
  (bind _asdmssave_game (cast `DMSSaveGame` _returnvalue))
  (bind _asbp_dmsplayer_state (cast `/Game/Gamemode/BP_DMSPlayerState` (`self.PlayerState`)))
  (bind _output_get (set `DMSPlayerState.PlayerCharacterData` (`DMSSaveGame.SavedCharacterData` _asdmssave_game) _asbp_dmsplayer_state))
  (`DMSPlayerState.SetCardDatas` _asbp_dmsplayer_state (`DMSSaveGame.SavedCardDatas` _asdmssave_game))
  (return (`DMSPlayerState.OriginalCardDatas` _asbp_dmsplayer_state) _output_get))

(fn `UserConstructionScript`
  (bind _returnvalue (`|GenericCreateObject` "/Game/Widgets/WB_TestHUD.WB_TestHUD_C"))
  (set `self.TestHUD` _returnvalue))