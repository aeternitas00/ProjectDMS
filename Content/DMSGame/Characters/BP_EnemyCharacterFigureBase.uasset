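; Base Blueprint for enemy character figures in a DMS game with Arkham attribute tags, adding a health readout and click interaction.
; On initialization it binds to the Damage attribute in AttributesComponent, then pushes the current value through UpdateHPWidget.
; UpdateHPWidget writes the rounded numeric value to a TextRender, so updates follow attribute changes without Tick.
; Clicking the hit box reveals the WB_EnemyCharacterInteraction widget held by the Widget component.
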(event `self.ReceiveBeginPlay`)

(event `self.ClickHitBox.OnClicked`
  (params (TouchedComponent :type "PrimitiveComponent Object Reference") (ButtonPressed :type "Key Structure"))
  (`Widget.SetVisibility` (cast `/Game/DMSGame/Widgets/CharacterInteraction/WB_EnemyCharacterInteraction` (`WidgetComponent.GetWidget` (`self.Widget`)) :!pure true) "SelfHitTestInvisible"))

(event `self.OnInitialized`
  (bind _returnvalue (`BlueprintGameplayTagLibrary.MakeLiteralGameplayTagContainer` (struct :`GameplayTags` (struct :`(TagName` "Attribute.Arkham.Character.Damage")))))
  (bind _attributescomponent (`self.AttributesComponent`))
  (`parent.OnInitialized`)
  (`DMSAttributeComponent.BindOnModifiedToAttribute` _attributescomponent _returnvalue (delegate `Update HP Widget`))
  (`self.Update HP Widget` (`DMSAttributeComponent.GetAttribute` _attributescomponent _returnvalue)))

(event `Update HP Widget`
  (params (Attribute :type "DMSAttribute Object Reference"))
  (bind _asdmsattribute_value_numeric (cast `DMSAttributeValue_Numeric` (`DMSAttribute.AttributeValue` Attribute)))
  (`TextRenderComponent.K2_SetText` (`self.TextRender`) (`KismetTextLibrary.Conv_IntToText` (`KismetMathLibrary.Round` (`DMSAttributeValue_Numeric.GetValue` _asdmsattribute_value_numeric)))))

(fn `UserConstructionScript`)