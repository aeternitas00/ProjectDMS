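; Test game mode for a card game that sets up the first player's hand and deck plus a row of dummy target cards on BeginPlay.
; SpawnCard creates and initializes random test cards, files them in the owner's DMSCardManagerComponent container and registers them with NotifyManager.
; Dummies spawn separately, register likewise, and get an HP attribute and text label, with a modify delegate intended to refresh the displayed value.
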(event `self.ReceiveBeginPlay`
  (bind _outitem (`KismetArrayLibrary.Array_Random` (`|MakeArray` "/Game/Card/TestCardDefinition.TestCardDefinition" "/Game/Card/TestCardDefinition2.TestCardDefinition2" "/Game/Card/TestCardDefinition3.TestCardDefinition3" "/Game/Card/TestCardDefinition4.TestCardDefinition4" :!type "DMSCardDefinition Object Reference")))
  (for _ (range 5)
    (bind _returnvalue (`self.SpawnCard` _outitem (`GameplayStatics.GetPlayerController` 0) "Hand"))
    (`self.SetActorHiddenInGame` _returnvalue false))
  (for _ (range 30)
    (bind _returnvalue_2 (`self.SpawnCard` _outitem (`GameplayStatics.GetPlayerController` 0) "Deck"))
    (`self.SetActorHiddenInGame` _returnvalue_2 true))
  (for _index (range 5)
    (bind _returnvalue_3 (`|SpawnActorFromClass` "/Game/Card/BP_Card.BP_Card_C" (`KismetMathLibrary.MakeTransform` (+ (* (`self.Dummy dist`) _index) (.location (`self.Dummy Spawn Transform`))) (.rotation (`self.Dummy Spawn Transform`)) (.scale (`self.Dummy Spawn Transform`))) "Undefined" "OverrideRootScale" self null))
    (`DMSCardBase.InitializeCard` _returnvalue_3 "/Game/Card/TestDummyCardDefinition.TestDummyCardDefinition")
    (`DMSNotifyManager.RegisterNotifyObject` (`self.NotifyManager`) (cast `DMSEffectorInterface` _returnvalue_3 :!pure true))
    (`self.SetActorHiddenInGame` _returnvalue_3 false) ; Temp
    (bind _returnvalue_4 (`|AddComponentByClass` _returnvalue_3 "/Script/ProjectDMSGame.DMSAttributeComponent"))
    (`DMSAttributeComponent.MakeAttribute` _returnvalue_4 "HP" 0.0)
    (`DMSAttributeComponent.BindOnModifiedToAttribute` _returnvalue_4 "HP" (delegate `커스텀이벤트`))
    (bind _returnvalue_5 (`AddComponent|NODE_AddTextRenderComponent-1` :`self` _returnvalue_3 :`bManualAttachment` true :`RelativeTransform` (`KismetMathLibrary.MakeTransform` (0.0 0.0 2.5) (struct :`Pitch` -90.0) (1.0 -1.0 1.0))))
    (bind _returnvalue_6 (`SceneComponent.K2_AttachToComponent` _returnvalue_5 (`/Game/Card/BP_Card.CardMesh` _returnvalue_3) "None" "KeepRelative" "KeepRelative" "KeepRelative" false))
    (if _returnvalue_6
      (`TextRenderComponent.K2_SetText` _returnvalue_5 "HP : 20")
      (`TextRenderComponent.SetHorizontalAlignment` _returnvalue_5 "EHTA_Center")
      (else
        (`KismetSystemLibrary.PrintString` "NO att")))))

(event `커스텀이벤트`
  (params (Attribute :type "DMSAttribute Object Reference"))
  (bind _returnvalue (`DMSAttribute.GetValue` Attribute))
  (`TextRenderComponent.K2_SetText` (stale `self.ReceiveBeginPlay` _returnvalue_5) (`KismetSystemLibrary.MakeLiteralText` (`KismetTextLibrary.Conv_StringToText` (`KismetStringLibrary.Concat_StrStr` "HP : " (`KismetStringLibrary.Conv_IntToString` (`KismetMathLibrary.Round` _returnvalue)))))))

(fn `SpawnCard`
  (params (iCardDef :type "DMSCardDefinition Object Reference") (iOwner :type "Actor Object Reference") (DefaultContainerName :type "Name (by ref)"))
  (returns (ReturnValue :type "DMSCardBase Object Reference"))
  (bind _returnvalue (`self.GetComponentByClass` iOwner "/Script/ProjectDMSGame.DMSCardManagerComponent"))
  (bind _returnvalue_2 (`|SpawnActorFromClass` "/Game/Card/BP_Card.BP_Card_C" (`self.Spawn Transform`) "Undefined" "OverrideRootScale" iOwner null))
  (`DMSCardBase.InitializeCard` _returnvalue_2 iCardDef)
  (`/Engine/EditorBlueprintResources/StandardMacros.IsValid` _returnvalue
    (:`Is Valid`
      (`DMSCardManagerComponent.AddCardtoContainer` _returnvalue (`|MakeArray` _returnvalue_2 :!type "DMSCardBase Object Reference") DefaultContainerName)
      (`DMSNotifyManager.RegisterNotifyObject` (`self.NotifyManager`) _returnvalue_2)
      (`self.SetActorHiddenInGame` _returnvalue_2 true) ; Temp
      (return _returnvalue_2))))

(fn `UserConstructionScript`)