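; Main game mode for the DMS game, which starts a match and provides helpers for players and their characters.
; BeginPlay runs setup after a short delay, then runs a start-game effect sequence through the SequenceManager with a finish callback.
; A phase-loop event drives the PhaseManager to generate, set up and start phases.
; Helpers return typed player states and controllers, and spawn characters from synchronously loaded definitions, linking them to their player state.
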(event `self.ReceiveBeginPlay`
  ;[1 1 1] TEST
  (`KismetSystemLibrary.Delay` 0.2)
  (`self.SetupDMSGame`)
  (`self.Start Game`))

(event `Initiate Phase Loop`
  (params (Dummy :type Boolean))
  (bind _phasemanager (`DMSGameStateBase.PhaseManager` (`self.GetDMSGameState`)))
  ;[1 1 1] TEST
  (`DMSPhaseManager.GeneratePhases` _phasemanager)
  (`DMSPhaseManager.SetupPhases` _phasemanager)
  (`DMSPhaseManager.InitiatePhaseLoop` _phasemanager))

(fn `Get DMS Players`
  (returns (OutActors :type "Array of /Game/DMSGame/Player/BP_DMSPlayerController Object Reference"))
  (locals (rv :type "Array of /Game/DMSGame/Player/BP_DMSPlayerController Object Reference"))
  (bind _rv (`local.rv`))
  (bind _asdmsgame_state (cast `DMSGameState` (`self.GetDMSGameState`)))
  (bind _returnvalue (`DMSGameState.GetDMSPlayerControllers` _asdmsgame_state))
  (for _array_element _returnvalue
    (bind _asbp_dmsplayer_controller (cast `/Game/DMSGame/Player/BP_DMSPlayerController` _array_element))
    (`KismetArrayLibrary.Array_Add` _rv _asbp_dmsplayer_controller))
  (return _rv))

(fn `Get DMS PlayerStates`
  (returns (OutActors :type "Array of /Game/DMSGame/Player/BP_DMSPlayerState Object Reference"))
  (locals (rv :type "Array of /Game/DMSGame/Player/BP_DMSPlayerState Object Reference"))
  (bind _rv (`local.rv`))
  (bind _asdmsgame_state (cast `DMSGameState` (`self.GetDMSGameState`)))
  (bind _returnvalue (`DMSGameState.GetDMSPlayers` _asdmsgame_state))
  (for _array_element _returnvalue
    (bind _asbp_dmsplayer_state (cast `/Game/DMSGame/Player/BP_DMSPlayerState` _array_element))
    (`KismetArrayLibrary.Array_Add` _rv _asbp_dmsplayer_state))
  (return _rv))

(fn `SpawnPlayerCharacter`
  (params (CharacterData :type "DMSPlayerCharacterData Structure") (Owner :type "/Game/DMSGame/Player/BP_DMSPlayerController Object Reference") (DefaultLocation :type "DMSLocationBase Object Reference"))
  (returns (SpawnedCharacter :type "/Game/DMSCore/Character/BP_CharacterBase Object Reference"))
  (locals (`Character spawn point` :type "Transform Structure" :default "-10.000000,0.000000,0.000000|0.000000,0.000000,0.000000|0.600000,0.600000,0.600000"))
  (bind _asbp_dmsplayer_state (`/Game/DMSGame/Player/BP_DMSPlayerController.GetDMSPlayerState` Owner))
  (bind _returnvalue (`KismetSystemLibrary.LoadAsset_Blocking` (`KismetSystemLibrary.GetSoftObjectReferenceFromPrimaryAssetId` (`.AssetID` (break `DMSPlayerCharacterData` CharacterData)))))
  (bind _asdmscharacter_definition (cast `DMSCharacterDefinition` _returnvalue))
  (bind _returnvalue_2 (`self.SpawnDMSGameActor_ID` _asdmscharacter_definition (`PlayerState.PlayerId` _asbp_dmsplayer_state) DefaultLocation (`local.Character spawn point`)))
  (bind _asbp_character_base (cast `/Game/DMSCore/Character/BP_CharacterBase` _returnvalue_2))
  (set `DMSPlayerState.CharacterRef` _asbp_character_base _asbp_dmsplayer_state)
  (return _asbp_character_base))

(fn `Start Game`
  (bind _returnvalue (`self.GetDMSGameState`))
  (bind _sequencemanager (`DMSGameStateBase.SequenceManager` (`self.GetDMSGameState`)))
  (bind _returnvalue_2 (`|GenericCreateObject` (`self.StartGameEffectNode`)))
  (bind _returnvalue_3 (`DMSSeqManager.RequestCreateSequence` _sequencemanager _returnvalue _returnvalue _returnvalue_2 (`|MakeArray`) null null))
  (`DMSSequence.AddToOnSequenceFinished` _returnvalue_3 (`|CreateDelegate` :!event `Initiate Phase Loop`))
  (`DMSSeqManager.RunSequence` _sequencemanager _returnvalue_3))

(fn `UserConstructionScript`)