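; BP_Card is a clickable card actor that shows the name and effect text from its card definition.
; Clicking the mesh passes the card to BP_DMSPlayerController's SelectObject.
; PopupInteractionWidget adds a screen-space widget component with a test play or activate widget, depending on whether the card's container is Hand or Play Area.
; CloseInteractionWidget destroys that component; an older viewport-projected play button remains but is never run.
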(event `self.ReceiveBeginPlay`
  (`parent.ReceiveBeginPlay`))

(event `Popup Interaction Widget`
  (`self.DisplayingWidget`
    (:`then`)
    (:`else`
      (`self.CardDefinition`
        (:`then`
          (bind _returnvalue (`|AddComponentByClass` self "/Script/UMG.WidgetComponent" false (`self.Relative Transform`)))
          (bind _output_get (set `self.DisplayingWidget` _returnvalue))
          (`WidgetComponent.SetDrawAtDesiredSize` _returnvalue true)
          (`WidgetComponent.SetWidgetSpace` _output_get "Screen")
          (switch `name` (`DMSCardContainerComponent.GetContainerName` (`self.OwningContainer`))
            (:`Hand`
              (bind _returnvalue_2 (`|CreateWidget` "/Game/Card/WB_TestPlayCard.WB_TestPlayCard_C" null self))
              (add `/Game/Card/WB_TestPlayCard.On Work Finished` _returnvalue_2 (`|CreateDelegate` :!event `Close Interaction Widget`))
              (`WidgetComponent.SetWidget` (`self.DisplayingWidget`) _returnvalue_2))
            (:`PlayArea`
              (bind _returnvalue_3 (`|CreateWidget` "/Game/Widgets/WB_TestActivateCard.WB_TestActivateCard_C" null self))
              (add `/Game/Widgets/WB_TestActivateCard.On Work Finished` _returnvalue_3 (`|CreateDelegate` :!event `Close Interaction Widget`))
              (`WidgetComponent.SetWidget` (`self.DisplayingWidget`) _returnvalue_3))))
        (:`else`
          (`KismetSystemLibrary.PrintString` "N/A Card"))))))

(event `Close Interaction Widget`
  (bind _displayingwidget (`self.DisplayingWidget`)
    (:`then`
      (`ActorComponent.K2_DestroyComponent` _displayingwidget))
    (:`else`)))

(event `self.CardMesh.OnClicked`
  (params (TouchedComponent :type "PrimitiveComponent Object Reference") (ButtonPressed :type "Key Structure"))
  (`DMSPlayerController.SelectObject` (cast `/Game/Player/BP_DMSPlayerController` (`GameplayStatics.GetPlayerController` 0) :!pure true) self))

(event `커스텀이벤트`
  (`KismetSystemLibrary.PrintString` (`KismetStringLibrary.Conv_BoolToString` (`self.HasAuthority`))))

(event `self.InitializeCard`
  (params (iCardDefinition :type "DMSCardDefinition Object Reference"))
  (`parent.InitializeCard` iCardDefinition)
  (`TextRenderComponent.K2_SetText` (`self.CardNameText`) (`DMSCardDefinition.CardName` (`self.CardDefinition`)))
  (`TextRenderComponent.K2_SetText` (`self.CardEffectText`) (`DMSCardDefinition.EffectText` (`self.CardDefinition`))))

(fn `Collapse Widget`)

(fn `UserConstructionScript`)