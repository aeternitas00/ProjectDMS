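; BP_CC_ThreatArea is a user card container for the threat area of a card game.
; MovementHelper teleports the container's cards into an evenly spaced row centered on CenterLoc, using Distance as the step between neighbors.
; Its matching container widget is the PlayArea of the card manager widget.
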(fn `Get Matching Container Widget Ref`
  (returns (`Out Widget` :type "/Game/DMSGame/Widgets/Card/Templates/WB_CardConatinerBase Object Reference"))
  (return (`/Game/DMSGame/Widgets/Card/Manager/WB_CardManager.PlayArea` (`self.Get Card Manager Widget`))))

(fn `MovementHelper`
  (bind _returnvalue (`self.GetCards`))
  (for (_array_element _array_index) _returnvalue
    (`Actor.K2_SetActorLocation` _array_element (+ (* _array_index (`self.Distance`)) (- (`self.CenterLoc`) (* (`self.Distance`) (- (`KismetArrayLibrary.Array_Length` _returnvalue) 1) (0.5 0.5 0.5)))) false true)))