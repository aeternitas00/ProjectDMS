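; Card container Blueprint for a play area that displays the cards it holds in an evenly spaced, centered row.
; When cards are added or removed, NewFunction teleports every held card to its slot, offset by Distance and centered on CenterLoc.
; Added cards are then made visible, while removed cards are hidden and teleported to the world origin.
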(event `self.ReceiveBeginPlay`)

(event `self.ReceiveTick`
  (params (DeltaSeconds :type "Float (single-precision)")))

(event `self.OnContainerAdded`
  (params (AddedCards :type "Array of DMSCardBase Object Reference (by ref)"))
  (`self.NewFunction`)
  (for _array_element AddedCards
    (`Actor.SetActorHiddenInGame` _array_element false)))

(event `self.OnContainerRemoved`
  (params (RemovedCards :type "Array of DMSCardBase Object Reference (by ref)"))
  (`self.NewFunction`)
  (for _array_element RemovedCards
    (`Actor.SetActorHiddenInGame` _array_element true)
    (`Actor.K2_SetActorLocation` _array_element (0.0 0.0 0.0) false true)))

(fn `NewFunction`
  (bind _returnvalue (`self.GetCards`))
  (for (_array_element _array_index) _returnvalue
    (`Actor.K2_SetActorLocation` _array_element (+ (* _array_index (`self.Distance`)) (- (`self.CenterLoc`) (* (`self.Distance`) (- (`KismetArrayLibrary.Array_Length` _returnvalue) 1) (0.5 0.5 0.5)))) false true)))