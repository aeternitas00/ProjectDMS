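; BP_TestLocation is a test location actor for the Arkham-tagged DMS game, showing its name, stats and revealed state.
; On initialization it sets the name text from location data and binds attribute events that fill a stat indicator widget and swap the revealed material.
; Clicking the hitbox prints the Clue value.
; Logic arranging entering actors into player and enemy grids is disconnected, leaving enter and leave events empty.
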(event `Update Revealed Material`
  (params (Attribute :type "DMSAttribute Object Reference"))
  (bind _staticmesh1 (`self.StaticMesh1`))
  (bind _asdmsattribute_value_boolean (cast `DMSAttributeValue_Boolean` (`DMSAttribute.AttributeValue` Attribute)))
  (if (`DMSAttributeValue_Boolean.GetValue` _asdmsattribute_value_boolean)
    (`PrimitiveComponent.SetMaterial` _staticmesh1 0 "/Game/CCGToolkit/Materials/LocRevealed.LocRevealed")
    (else
      (`PrimitiveComponent.SetMaterial` _staticmesh1 0 "/Game/CCGToolkit/Materials/LocUnrevealed.LocUnrevealed"))))

(event `Add Attribute Widget`
  (params (Attribute :type "DMSAttribute Object Reference"))
  (bind _aswb_stat_indicator_list (cast `/Game/DMSGame/Widgets/WB_StatIndicatorList` (`WidgetComponent.GetWidget` (`self.StatIndicator`))))
  (`/Game/DMSGame/Widgets/WB_StatIndicatorList.Add Attribute` _aswb_stat_indicator_list Attribute))

(event `self.OnInitialized`
  (`DMSAttributeComponent.BindOnAttributeAdded` (`self.AttributeComponent`) (delegate `Add Attribute Widget`))
  (`parent.OnInitialized`)
  (`TextRenderComponent.K2_SetText` (`self.TextRender`) (`KismetTextLibrary.Conv_NameToText` (`DMSLocationData.LocationName` (cast `DMSLocationData` (`self.OriginalData`) :!pure true))))
  (`DMSAttributeComponent.BindOnModifiedToAttribute` (`self.AttributeComponent`) (`BlueprintGameplayTagLibrary.MakeLiteralGameplayTagContainer` (struct :`GameplayTags` (struct :`(TagName` "Attribute.Arkham.Location.Revealed")))) (delegate `Update Revealed Material`)))

(event `self.OnActorEntered`
  (params (Locatable :type "DMSLocatableInterface Interface (by ref)")))

(event `self.OnActorLeaved`
  (params (Locatable :type "DMSLocatableInterface Interface (by ref)")))

(event `self.ClickHitBox.OnClicked`
  (params (TouchedComponent :type "PrimitiveComponent Object Reference") (ButtonPressed :type "Key Structure"))
  (bind _asdmsattribute_value_numeric (cast `DMSAttributeValue_Numeric` (`DMSAttributeComponent.GetAttributeValue` (`self.AttributeComponent`) (`BlueprintGameplayTagLibrary.MakeLiteralGameplayTagContainer` (struct :`GameplayTags` (struct :`(TagName` "Attribute.Arkham.Common.Clue")))) true)))
  (`KismetSystemLibrary.PrintString` (`KismetStringLibrary.Conv_DoubleToString` (`DMSAttributeValue_Numeric.GetValue` _asdmsattribute_value_numeric))))

(fn `UpdateChildsOffset`
  (params (Array :type "Array of Actor Object Reference"))
  (locals (DistanceX :type "Vector Structure" :default (0.0 140.0 0.0)) (NumPerRow :type Integer :default 3) (DistanceY :type "Vector Structure" :default (-140.0 0.0 0.0)))
  (bind _numperrow (`local.NumPerRow`))
  (for (_array_element _array_index) Array
    (`self.K2_SetActorRelativeLocation` _array_element (+ (* (`local.DistanceX`) (mod _array_index _numperrow)) (* (`local.DistanceY`) (`KismetMathLibrary.Conv_IntToVector` (/ _array_index _numperrow)))) false true)))

(fn `UserConstructionScript`)