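; Phase manager Blueprint for a DMS game mode that reacts to phase changes in a looping chain of phases.
; SetupPhases walks the NextPhase links from the current phase until it wraps around, binding start and end delegates on each.
; When a phase starts, it updates the HUD phase widget through the player controller and runs the phase's effect node as a sequence via the DMS sequence manager.
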(event `Default OnPhaseStarted`
  (params (CurrentPhase :type "DMSPhase Object Reference"))
  (`self.UpdatePhaseWidget` CurrentPhase)
  (`self.NewMacro` CurrentPhase))

(event `Default OnPhaseEnded`
  (params (CurrentPhase :type "DMSPhase Object Reference")))

(event `self.UpdatePhaseWidget`
  (params (iPhase :type "DMSPhase Object Reference"))
  (bind _asbp_dmsplayer_controller (cast `/Game/Player/BP_DMSPlayerController` (`GameplayStatics.GetPlayerController` 0)))
  (`/Game/Widgets/WB_TestHUD.Update Phase Widget` (`/Game/Player/BP_DMSPlayerController.TestHUD` _asbp_dmsplayer_controller) iPhase))

(event `Set Active of Phase widget`
  (params (iActive :type Boolean))
  (bind _asbp_dmsplayer_controller (cast `/Game/Player/BP_DMSPlayerController` (`GameplayStatics.GetPlayerController` 0)))
  (`/Game/Widgets/WB_TestHUD.Set Active of Phase widget` (`/Game/Player/BP_DMSPlayerController.TestHUD` _asbp_dmsplayer_controller) iActive))

(fn `SetupPhases`
  (locals (It :type "DMSPhase Object Reference"))
  (bind _returnvalue (`self.GetCurrentPhase`))
  (`/Engine/EditorBlueprintResources/StandardMacros.IsValid` _returnvalue
    (:`Is Valid`
      (bind _output_get (set `local.It` _returnvalue))
      (add `DMSPhase.OnPhaseStarted` _output_get (`|CreateDelegate` :!event `Default OnPhaseStarted`) :!label _label)
      (add `DMSPhase.OnPhaseEnded` _output_get (`|CreateDelegate` :!event `Default OnPhaseEnded`))
      (bind _output_get_2 (set `local.It` (`DMSPhase.NextPhase` _output_get)))
      (bind _returnvalue_2 (`self.GetCurrentPhase`))
      (if (== _output_get_2 _returnvalue_2)
        (return)
        (else
          (goto _label))))
    (:`Is Not Valid`
      (return))))