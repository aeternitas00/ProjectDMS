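; Hand card container that links the game's card data to the player's hand UI.
; On BeginPlay it takes the existing Hand widget from the card manager widget, sets itself as that widget's container reference and adds its current cards to it.
; An unused legacy graph instead creates a WB_PlayerHand widget dynamically and anchors it full-screen on the test HUD canvas.
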(event `self.ReceiveBeginPlay`
  (bind _output_get (set `self.ContainerWidgetRef` (`/Game/DMSGame/Widgets/Card/WB_CardManager.Hand` (`self.Get Card Manager Widget`))))
  (set `/Game/DMSGame/Widgets/Card/WB_CardConatinerBase.Container_Ref` self _output_get)
  (`/Game/DMSGame/Widgets/Card/WB_CardConatinerBase.Add cards` _output_get (`self.GetCards`)))