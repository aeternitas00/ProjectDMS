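; Card container Blueprint for a player's hand, linking the container to its UI widget.
; Its only live logic is GetMatchingContainerWidgetRef, which returns the Hand widget from the card manager widget.
; Unconnected EventGraph nodes would bind that widget and add the cards directly.
; An unused legacy graph instead creates WB_PlayerHand dynamically and stretches it across the test HUD canvas.
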(fn `Get Matching Container Widget Ref`
  (returns (`Out Widget` :type "/Game/DMSGame/Widgets/Card/Templates/WB_CardConatinerBase Object Reference"))
  (return (`/Game/DMSGame/Widgets/Card/Manager/WB_CardManager.Hand` (`self.Get Card Manager Widget`))))