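; BP_PlayerCharacterBase is a player character base Blueprint that shows a character-move widget when clicked.
; On BeginPlay it passes itself as CharacterRef to the WB_CharacterMove held by its Widget component.
; Clicking the ClickHitBox component makes that widget visible as SelfHitTestInvisible, then initializes it with the result of GetCurrentLocation.
; Overlap and Tick events are empty, as is the construction script.
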(event `self.ReceiveBeginPlay`
  (set `/Game/DMSGame/Widgets/CharacterInteraction/WB_CharacterMove.CharacterRef` self (cast `/Game/DMSGame/Widgets/CharacterInteraction/WB_CharacterMove` (`WidgetComponent.GetWidget` (`self.Widget`)) :!pure true)))

(event `self.ClickHitBox.OnClicked`
  (params (TouchedComponent :type "PrimitiveComponent Object Reference") (ButtonPressed :type "Key Structure"))
  (bind _aswb_character_move (cast `/Game/DMSGame/Widgets/CharacterInteraction/WB_CharacterMove` (`WidgetComponent.GetWidget` (`self.Widget`)) :!pure true))
  (`Widget.SetVisibility` _aswb_character_move "SelfHitTestInvisible")
  (bind _returnvalue (`DMSLocatableInterface.GetCurrentLocation`))
  (`/Game/DMSGame/Widgets/CharacterInteraction/WB_CharacterMove.Initialize` _aswb_character_move _returnvalue))

(fn `UserConstructionScript`)