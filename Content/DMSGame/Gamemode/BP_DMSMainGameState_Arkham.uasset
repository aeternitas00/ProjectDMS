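; Main game state for the Arkham game mode on the DMS framework, managing the chaos token bag and game-wide stat display.
; On SetupDefaults it spawns hidden token actors from definitions saved in "TestSlot" and puts them in the ChaosTokenBag container.
; It adds existing and newly added numeric attributes to player controllers' test HUDs.
; CreateChaosTokenDrawSeq requests a token-draw sequence under a given parent, using an effect node built at construction.
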(event `self.SetupDefaults`
  (bind _attributecomponent (`self.AttributeComponent`))
  (`parent.SetupDefaults`)
  (`self.SpawnChaosTokens`)
  (for _array_element (`DMSAttributeComponent.Attributes` _attributecomponent)
    (`self.Register to HUD` _array_element))
  (`DMSAttributeComponent.BindOnAttributeAdded` _attributecomponent (delegate `Register to HUD`)))

(event `Register to HUD`
  (params (Attribute :type "DMSAttribute Object Reference"))
  (for _index (range (`GameplayStatics.GetNumPlayerControllers`))
    (bind _asbp_dmsplayer_controller (cast `/Game/DMSGame/Player/BP_DMSPlayerController` (`GameplayStatics.GetPlayerController` _index)))
    (cast `DMSAttributeValue_Numeric` (`DMSAttribute.AttributeValue` Attribute))
    (`/Game/DMSGame/Widgets/WB_StatIndicatorList.Add Attribute` (`/Game/DMSGame/Widgets/WB_TestHUD.GameStateStat` (`/Game/DMSGame/Player/BP_DMSPlayerController.TestHUD` _asbp_dmsplayer_controller)) Attribute)))

(fn `CreateChaosTokenDrawSeq`
  (params (ParentSeq :type "DMSSequence Object Reference"))
  (returns (ReturnValue :type "DMSSequence Object Reference"))
  (bind _returnvalue (`DMSSeqManager.RequestCreateSequence` (`DMSCoreFunctionLibrary.GetDMSSequenceManager` self) self self (`DMSEffectNodeWrapper.GetEffectNodeBP` (`.EffectNode` (break `DMSInstancedEffectNode` (`self.DrawChaosTokenEN`)))) (`|MakeArray`) true ParentSeq))
  (return _returnvalue))

(fn `SpawnChaosTokens`
  (locals (LocalObjects :type "Array of DMSSpawnableBase Object Reference"))
  (bind _returnvalue (`GameplayStatics.LoadGameFromSlot` "TestSlot"))
  (bind _asdmssave_game (cast `DMSSaveGame` _returnvalue))
  (for _array_element (`DMSSaveGame.SavedChaosTokenDatas` _asdmssave_game)
    (bind _asdmschaos_token_definition (cast `DMSChaosTokenDefinition` (`KismetSystemLibrary.GetObjectFromPrimaryAssetId` _array_element)))
    (bind _asdmsgame_mode (cast `DMSGameMode` (`GameplayStatics.GetGameMode`)))
    (bind _returnvalue_2 (`DMSGameMode.SpawnDMSGameActor_ID` _asdmsgame_mode _asdmschaos_token_definition -1 null (`KismetMathLibrary.MakeTransform` (0.0 0.0 0.0))))
    (`KismetArrayLibrary.Array_Add` (`local.LocalObjects`) _returnvalue_2)
    (`self.SetActorHiddenInGame` _returnvalue_2 true))
  (`DMSContainerManagerComponent.AddObjectstoContainer` (`self.ContainerManagerComponent`) (`local.LocalObjects`) (`BlueprintGameplayTagLibrary.MakeLiteralGameplayTag` (struct :`TagName` "Field.Arkham.ChaosTokenBag"))))

(fn `UserConstructionScript`
  (`|GenericCreateObject` "/Game/DMSGame/Gamemode/GM_Effects/EN_DrawChaosToken.EN_DrawChaosToken_C"))