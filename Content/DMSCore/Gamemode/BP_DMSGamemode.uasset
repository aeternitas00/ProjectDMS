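; Game mode for the DMS card game framework that sets up the match and spawns cards and player characters.
; PostLogin triggers client HUD setup and, as a test shortcut, starts game setup once two players join.
; StartGame runs a sequence through the game state's SequenceManager with a finish callback; InitiatePhaseLoop has PhaseManager generate, set up and start phases.
; Characters load synchronously from asset IDs and are linked to their owner's player state.
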(event `self.ReceiveBeginPlay`
  (`KismetSystemLibrary.Delay` 0.2))

(event `Initiate Phase Loop`
  (params (Dummy :type Boolean))
  (bind _phasemanager (`DMSGameStateBase.PhaseManager` (`self.GetDMSGameState`)))
  (`DMSPhaseManager.GeneratePhases` _phasemanager)
  (`DMSPhaseManager.SetupPhases` _phasemanager)
  (`DMSPhaseManager.InitiatePhaseLoop` _phasemanager))

(event `self.K2_PostLogin`
  (params (NewPlayer :type "PlayerController Object Reference"))
  (`parent.K2_PostLogin` NewPlayer)
  (bind _asbp_dmsplayer_controller (cast `/Game/DMSGame/Player/BP_DMSPlayerController` NewPlayer))
  (`/Game/DMSGame/Player/BP_DMSPlayerController.Client HUD Works` _asbp_dmsplayer_controller)
  (`KismetSystemLibrary.PrintString` (`KismetStringLibrary.Concat_StrStr` (`KismetSystemLibrary.GetObjectName` NewPlayer) " pl " (`KismetStringLibrary.Conv_BoolToString` (`self.HasAuthority` NewPlayer))) true true (struct :`G` 0.66 :`B` 1.0 :`A` 1.0) 20.0)
  ;[1 1 1] for test
  (if (== (`KismetArrayLibrary.Array_Length` (`GameStateBase.PlayerArray` (`GameplayStatics.GetGameState`))) 2)
    (`self.SetupDMSGame`)))

(event `self.OnAllPlayerReady`)

(event `Start Game`
  (bind _returnvalue (`self.GetDMSGameState`))
  (bind _sequencemanager (`DMSGameStateBase.SequenceManager` (`self.GetDMSGameState`)))
  (bind _returnvalue_2 (`|GenericCreateObject` (`self.Effect Node`)))
  (bind _returnvalue_3 (`DMSSeqManager.RequestCreateSequence` _sequencemanager _returnvalue _returnvalue _returnvalue_2 (`|MakeArray`) null null))
  (`DMSSequence.AddToOnSequenceFinished` _returnvalue_3 (`|CreateDelegate` :!event `Initiate Phase Loop`))
  (`DMSSeqManager.RunSequence` _sequencemanager _returnvalue_3))

(fn `Get DMS Players`
  (returns (OutActors :type "Array of /Game/DMSGame/Player/BP_DMSPlayerController Object Reference"))
  (locals (rv :type "Array of /Game/DMSGame/Player/BP_DMSPlayerController Object Reference"))
  (bind _rv (`local.rv`))
  (bind _asdmsgame_state (cast `DMSGameState` (`self.GetDMSGameState`)))
  (bind _returnvalue (`DMSGameState.GetDMSPlayerControllers` _asdmsgame_state))
  (for _array_element _returnvalue
    (bind _asbp_dmsplayer_controller (cast `/Game/DMSGame/Player/BP_DMSPlayerController` _array_element))
    (`KismetArrayLibrary.Array_Add` _rv _asbp_dmsplayer_controller))
  (return _rv))

(fn `Get DMS PlayerStates`
  (returns (OutActors :type "Array of /Game/DMSGame/Player/BP_DMSPlayerState Object Reference"))
  (locals (rv :type "Array of /Game/DMSGame/Player/BP_DMSPlayerState Object Reference"))
  (bind _rv (`local.rv`))
  (bind _asdmsgame_state (cast `DMSGameState` (`self.GetDMSGameState`)))
  (bind _returnvalue (`DMSGameState.GetDMSPlayers` _asdmsgame_state))
  (for _array_element _returnvalue
    (bind _asbp_dmsplayer_state (cast `/Game/DMSGame/Player/BP_DMSPlayerState` _array_element))
    (`KismetArrayLibrary.Array_Add` _rv _asbp_dmsplayer_state))
  (return _rv))

(fn `SpawnCard`
  (params (CardData :type "DMSCardData Structure (by ref)") (OwnerID :type Integer) (DefaultContainerName :type "Name (by ref)"))
  (returns (ReturnValue :type "DMSCardBase Object Reference"))
  (bind _returnvalue (`parent.SpawnCard` CardData OwnerID DefaultContainerName))
  (return _returnvalue))

(fn `SpawnPlayerCharacter`
  (params (CharacterData :type "DMSPlayerCharacterData Structure") (Owner :type "/Game/DMSGame/Player/BP_DMSPlayerController Object Reference") (DefaultLocation :type "DMSLocationBase Object Reference"))
  (returns (SpawnedCharacter :type "/Game/DMSCore/Character/BP_CharacterBase Object Reference"))
  (locals (`Character spawn point` :type "Transform Structure" :default "-10.000000,0.000000,0.000000|0.000000,0.000000,0.000000|0.600000,0.600000,0.600000"))
  (bind _asbp_dmsplayer_state (`/Game/DMSGame/Player/BP_DMSPlayerController.GetDMSPlayerState` Owner))
  (bind _returnvalue (`KismetSystemLibrary.LoadAsset_Blocking` (`KismetSystemLibrary.GetSoftObjectReferenceFromPrimaryAssetId` (`.AssetID` (break `DMSPlayerCharacterData` CharacterData)))))
  (bind _asdmscharacter_definition (cast `DMSCharacterDefinition` _returnvalue))
  (bind _returnvalue_2 (`self.SpawnDMSGameActor_ID` _asdmscharacter_definition (`PlayerState.PlayerId` _asbp_dmsplayer_state) DefaultLocation (`local.Character spawn point`)))
  (bind _asbp_character_base (cast `/Game/DMSCore/Character/BP_CharacterBase` _returnvalue_2))
  (set `DMSPlayerState.CharacterRef` _asbp_character_base _asbp_dmsplayer_state)
  (return _asbp_character_base))

(fn `UserConstructionScript`)