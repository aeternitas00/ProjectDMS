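; Game mode for the DMS card game that sets up a test match and starts the PhaseManager's phase loop.
; On BeginPlay it spawns random cards into the first player's Hand and hidden Deck through the card manager component.
; It also spawns a row of dummy cards, each with an HP attribute and text label refreshed through a modification delegate.
; All spawned cards register with the NotifyManager.
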(event `커스텀이벤트`
  (params (Attribute :type "DMSAttribute Object Reference"))
  (bind _returnvalue (`DMSAttribute.GetValue` Attribute))
  (for _array_element (`self.GetComponentsByTag` (cast `Actor` (`KismetSystemLibrary.GetOuterObject` (`KismetSystemLibrary.GetOuterObject` Attribute)) :!pure true) "/Script/Engine.TextRenderComponent" "HP")
    (`TextRenderComponent.K2_SetText` _array_element (`KismetSystemLibrary.MakeLiteralText` (`KismetTextLibrary.Conv_StringToText` (`KismetStringLibrary.Concat_StrStr` "HP : " (`KismetStringLibrary.Conv_IntToString` (`KismetMathLibrary.Round` _returnvalue))))))))

(event `self.ReceiveBeginPlay`
  (bind _returnvalue (`BlueprintGameplayTagLibrary.MakeLiteralGameplayTag` (struct :`TagName` "Attribute.HP")))
  (bind _outitem (`KismetArrayLibrary.Array_Random` (`self.Array`)))
  (for _ (range 5)
    (bind _returnvalue_2 (`self.SpawnCard` _outitem (`GameplayStatics.GetPlayerController` 0) "Hand"))
    (`self.SetActorHiddenInGame` _returnvalue_2 false))
  (for _ (range 10)
    (bind _returnvalue_3 (`self.SpawnCard` _outitem (`GameplayStatics.GetPlayerController` 0) "Deck"))
    (`self.SetActorHiddenInGame` _returnvalue_3 true))
  (for _index (range 5)
    (bind _returnvalue_4 (`|SpawnActorFromClass` "/Game/Card/BP_Card.BP_Card_C" (`KismetMathLibrary.MakeTransform` (+ (* (`self.Dummy dist`) _index) (.location (`self.Dummy Spawn Transform`))) (.rotation (`self.Dummy Spawn Transform`)) (.scale (`self.Dummy Spawn Transform`))) "Undefined" "OverrideRootScale" self null))
    (`self.SetActorHiddenInGame` _returnvalue_4 false) ; Temp
    (bind _returnvalue_5 (`|AddComponentByClass` _returnvalue_4 "/Script/ProjectDMSGame.DMSAttributeComponent"))
    (`DMSAttributeComponent.MakeAttribute` _returnvalue_5 _returnvalue 20.0)
    (`DMSAttributeComponent.BindOnModifiedToAttribute` _returnvalue_5 _returnvalue (`|CreateDelegate` :!event `커스텀이벤트`))
    (bind _returnvalue_6 (`AddComponent|NODE_AddTextRenderComponent-1` :`self` _returnvalue_4 :`bManualAttachment` true :`RelativeTransform` (`KismetMathLibrary.MakeTransform` (0.0 0.0 2.5) (struct :`Pitch` -90.0) (1.0 -1.0 1.0))))
    (bind _returnvalue_7 (`SceneComponent.K2_AttachToComponent` _returnvalue_6 (`/Game/Card/BP_Card.CardMesh` _returnvalue_4) "None" "KeepRelative" "KeepRelative" "KeepRelative" false))
    (`KismetArrayLibrary.Array_Add` (`ActorComponent.ComponentTags` _returnvalue_6) "HP")
    (if _returnvalue_7
      (`TextRenderComponent.K2_SetText` _returnvalue_6 "HP : 20")
      (`TextRenderComponent.SetHorizontalAlignment` _returnvalue_6 "EHTA_Center")
      (`DMSCardBase.InitializeCard` _returnvalue_4 "/Game/Card/TestDummyCardDefinition.TestDummyCardDefinition")
      (`DMSNotifyManager.RegisterNotifyObject` (`self.NotifyManager`) (cast `DMSEffectorInterface` _returnvalue_4 :!pure true))
      (else
        (`KismetSystemLibrary.PrintString` "NO att"))))
  (`self.Initiate Phase Loop`))

(event `Initiate Phase Loop`
  (bind _phasemanager (`self.PhaseManager`))
  (`DMSPhaseManager.GeneratePhases` _phasemanager)
  (`DMSPhaseManager.SetupPhases` _phasemanager)
  (`DMSPhaseManager.InitiatePhaseLoop` _phasemanager))

(fn `Get DMS Players`
  (returns (OutActors :type "Array of /Game/Player/BP_DMSPlayerController Object Reference"))
  (bind _outactors (`GameplayStatics.GetAllActorsOfClass` "/Game/Player/BP_DMSPlayerController.BP_DMSPlayerController_C"))
  (return _outactors))

(fn `SpawnCard`
  (params (iCardDef :type "DMSCardDefinition Object Reference") (iOwner :type "Actor Object Reference") (DefaultContainerName :type "Name (by ref)"))
  (returns (ReturnValue :type "DMSCardBase Object Reference"))
  (bind _returnvalue (`self.GetComponentByClass` iOwner "/Script/ProjectDMSGame.DMSCardManagerComponent"))
  (bind _returnvalue_2 (`|SpawnActorFromClass` "/Game/Card/BP_Card.BP_Card_C" (`self.Spawn Transform`) "Undefined" "OverrideRootScale" iOwner null))
  (`DMSCardBase.InitializeCard` _returnvalue_2 iCardDef)
  (`/Engine/EditorBlueprintResources/StandardMacros.IsValid` _returnvalue
    (:`Is Valid`
      (`DMSCardManagerComponent.AddCardtoContainer` _returnvalue (`|MakeArray` _returnvalue_2 :!type "DMSCardBase Object Reference") DefaultContainerName)
      (`DMSNotifyManager.RegisterNotifyObject` (`self.NotifyManager`) _returnvalue_2)
      (`self.SetActorHiddenInGame` _returnvalue_2 true) ; Temp
      (return _returnvalue_2))))

(fn `Test`
  (params (NewParam :type "DMSPhase Object Reference")))

(fn `UserConstructionScript`)