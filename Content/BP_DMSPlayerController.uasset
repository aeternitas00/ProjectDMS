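; BP_DMSPlayerController is a player controller that creates the WB_Test widget on BeginPlay and adds it to the viewport.
; PlayCard and Tick events are empty stubs.
; An unconnected chain, which never runs, spawns two BP_Card actors, adds them to the "Hand" container through CardManagerComponent and prints a message.
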(event `self.ReceiveBeginPlay`
  (bind _returnvalue (`|CreateWidget` "/Game/Widgets/WB_Test.WB_Test_C" self))
  (`UserWidget.AddToViewport` _returnvalue 0))

(event `Play Card`
  (params (InCard :type "DMSCardBase Object Reference")))

(event `self.ReceiveTick`
  (params (DeltaSeconds :type "Float (single-precision)")))

(fn `UserConstructionScript`)