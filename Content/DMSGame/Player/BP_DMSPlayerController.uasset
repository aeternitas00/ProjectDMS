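; Player controller for the DMS card game, handling the HUD, card selection and card play.
; It constructs a test HUD, shows it with game-and-UI input, and moves the interaction popup between selected cards the player owns.
; A test PlayCard event runs the player state's default "PlayCard" effect through the sequence manager, targeting the card.
; A load function copies saved character and card data from the default save slot into the player state.
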(event `self.ReceiveBeginPlay`
  (`parent.ReceiveBeginPlay`))

(event `self.SetupHUDWidgets`
  (`/Game/DMSGame/Widgets/WB_TestHUD.Setup Subwidget` (`self.TestHUD`)))

(event `self.CreateHUDWidgets`
  (bind _testhud (`self.TestHUD`))
  (`UserWidget.SetOwningPlayer` _testhud self)
  (`UserWidget.AddToViewport` _testhud 0)
  (`WidgetBlueprintLibrary.SetInputMode_GameAndUIEx` self _testhud "DoNotLock" false))

(event `self.PlayCard`
  (params (Card :type "DMSCardBase Object Reference"))
  (bind _asbp_dmsplayer_state (`self.GetDMSPlayerState`))
  (bind _returnvalue (`DMSCoreFunctionLibrary.GetDMSSequenceManager`))
  (bind _returnvalue_2 (`DMSSeqManager.RequestCreateSequence` _returnvalue _asbp_dmsplayer_state _asbp_dmsplayer_state (`BlueprintMapLibrary.Map_Find` (`DMSPlayerState.DefaultBasicActions` (`self.GetDMSPlayerState`)) "PlayCard") (`|MakeArray` (cast `DMSEffectorInterface` Card :!pure true)) null null))
  (`DMSSeqManager.RunSequence` _returnvalue _returnvalue_2))

(event `self.OnSelectedObject`
  (params (FormerObject :type "Object Object Reference"))
  (`|ExecutionSequence`
    (:`then_0`
      (bind _asbp_card (`self.Check Object Is My Card` FormerObject)
        (:`then`
          (`/Game/DMSCore/Card/BP_Card.Close Interaction Widget` _asbp_card))))
    (:`then_1`
      (bind _asbp_card_2 (`self.Check Object Is My Card` (`self.SelectingObject`))
        (:`then`
          (`/Game/DMSCore/Card/BP_Card.Popup Interaction Widget` _asbp_card_2))))))

(fn `GetDMSPlayerState`
  (returns (`AsBP DMSPlayer State` :type "/Game/DMSGame/Player/BP_DMSPlayerState Object Reference"))
  (return (cast `/Game/DMSGame/Player/BP_DMSPlayerState` (`self.PlayerState`) :!pure true)))

(fn `Load Client Save game`
  (returns (`Saved Card Datas` :type "Array of DMSCardData Structure") (`Player Character Data` :type "DMSPlayerCharacterData Structure"))
  (bind _returnvalue (`GameplayStatics.LoadGameFromSlot` (`self.Default Slot Name`)))
  (bind _asdmssave_game (cast `DMSSaveGame` _returnvalue))
  (bind _asbp_dmsplayer_state (cast `/Game/DMSGame/Player/BP_DMSPlayerState` (`self.PlayerState`)))
  (bind _output_get (set `DMSPlayerState.PlayerCharacterData` (`DMSSaveGame.SavedCharacterData` _asdmssave_game) _asbp_dmsplayer_state))
  (`DMSPlayerState.SetCardDatas` _asbp_dmsplayer_state (`DMSSaveGame.SavedCardDatas` _asdmssave_game))
  (return (`DMSPlayerState.OriginalCardDatas` _asbp_dmsplayer_state) _output_get))

(fn `UserConstructionScript`
  (bind _returnvalue (`|GenericCreateObject` "/Game/DMSGame/Widgets/WB_TestHUD.WB_TestHUD_C"))
  (set `self.TestHUD` _returnvalue))